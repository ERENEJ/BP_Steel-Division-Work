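; Soldier component that handles fast-roping down from a helicopter.
; On activation it disables player input and fall damage, lowers gravity, then pins the soldier's XY to the rope component each tick while Z descends freely.
; It deactivates on landing, rope loss or a 7-second failsafe from BeginPlay.
; Deactivation restores control and physics, clears rappel animations and destroys the component if the animation checks pass.
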(event `OnDeactivate`
  (params (Component :type "ActorComponent Object Reference"))
  ;[1 1 1] Removed for testing class defaults values reverted
  (bind _assqsoldier (cast `SQSoldier` (`self.GetOwner` Component)))
  (set `CharacterMovementComponent.GravityScale` 1.0 (`Character.CharacterMovement` _assqsoldier))
  (set `SQSoldier.FallingDamageMultiplier` (defaults `/Steel_Division/Blueprints/Components/fast_ropes/BP_FastRopeComponent` (`GameplayStatics.GetObjectClass` _assqsoldier)) _assqsoldier)
  (bind _asbp_player_controller (cast `/Game/Blueprints/BP_PlayerController` (`Pawn.GetController` _assqsoldier) :!pure true))
  (`/Engine/EditorBlueprintResources/StandardMacros.IsValid` _asbp_player_controller
    (:`Is Valid`
      (`Actor.EnableInput` _asbp_player_controller _asbp_player_controller)
      (`Controller.SetIgnoreLookInput` _asbp_player_controller false))))

(event `self.ReceiveBeginPlay`
  (add `self.OnComponentActivated` (delegate `CustomEvent_0`))
  (`self.SetComponentTickEnabled` false)
  (add `self.OnComponentDeactivated` (delegate `On_Deactivated`))
  ;[1 1 1] testing the case when soldiers dies on rope / Fail safe
  (`KismetSystemLibrary.Delay` 7.0)
  (`self.Deactivate`))

(event `On_Deactivated` :!signature `self.OnComponentDeactivated`
  (params (Component :type "ActorComponent Object Reference"))
  (bind _returnvalue (`Pawn.GetController` (`self.SQSoldier`)))
  (bind _asbp_player_controller (cast `/Game/Blueprints/BP_PlayerController` _returnvalue :!pure true))
  (`/Engine/EditorBlueprintResources/StandardMacros.IsValid` (`self.SQSoldier`)
    (:`Is Valid`
      (`/Engine/EditorBlueprintResources/StandardMacros.IsValid` _asbp_player_controller
        (:`Is Valid`
          (`Actor.EnableInput` _asbp_player_controller _asbp_player_controller)
          (`Controller.SetIgnoreLookInput` _returnvalue false))
        (:`Is Not Valid`
          _))
      (set `CharacterMovementComponent.GravityScale` 1.0 (`Character.CharacterMovement` (`self.SQSoldier`)))
      (set `SQSoldier.FallingDamageMultiplier` 50.0 (`self.SQSoldier`))
      (`KismetSystemLibrary.K2_ClearAndInvalidateTimerHandle` (stale `CustomEvent_0` _returnvalue))
      (`KismetSystemLibrary.K2_ClearAndInvalidateTimerHandle` (stale `CustomEvent_0` _returnvalue_2))
      ;[1 1 1] to deactivate fast rope anim cancel with rope
      (bind _assd_bp_mutable_soldier (cast `/Steel_Division/Blueprints/Mutablesoldiers/SD_BP_MutableSoldier` (`self.SQSoldier`)))
      (`/Steel_Division/Blueprints/Mutablesoldiers/SD_BP_MutableSoldier.Server Event Landed` _assd_bp_mutable_soldier)
      (bind _returnvalue_2 (`SkeletalMeshComponent.GetAnimInstance` (`SQSoldierNew.UpperMesh1P` _assd_bp_mutable_soldier)))
      (`/Engine/EditorBlueprintResources/StandardMacros.IsValid` _returnvalue_2
        (:`Is Valid`
          (bind _assd_bp_1p_upper (cast `/Steel_Division/Animations/SD_BP_1P_Upper` _returnvalue_2))
          (set `/Steel_Division/Animations/SD_BP_1P_Upper.Is Rappeling` false _assd_bp_1p_upper)
          (bind _returnvalue_3 (`SkeletalMeshComponent.GetAnimInstance` (`Character.Mesh` _assd_bp_mutable_soldier)))
          (`/Engine/EditorBlueprintResources/StandardMacros.IsValid` _returnvalue_3
            (:`Is Valid`
              (`AnimInstance.StopSlotAnimation` _returnvalue_3 0.25 "FullBody")
              (bind _assd_bp_3p_3 (cast `/Steel_Division/Animations/SD_BP_3P_3` _returnvalue_3))
              (set `/Steel_Division/Animations/SD_BP_3P_3.Is Rappeling` false _assd_bp_3p_3)
              (`self.K2_DestroyComponent`))
            (:`Is Not Valid`)))
        (:`Is Not Valid`)))
    (:`Is Not Valid`
      (`KismetSystemLibrary.PrintString` "sq soldier is not valid on comp deactivated" true true (struct :`R` 1.0 :`A` 1.0) 20.0))))

(event `CustomEvent_0` :!signature `self.OnComponentActivated`
  (params (Component :type "ActorComponent Object Reference") (bReset :type Boolean))
  (bind _charactermovement (`Character.CharacterMovement` (`self.SQSoldier`)))
  (bind _asbp_player_controller (cast `/Game/Blueprints/BP_PlayerController` (`Pawn.GetController` (`self.SQSoldier`)) :!pure true))
  (bind _assqsoldier (cast `SQSoldier` (`self.GetOwner` Component))
    (:`then`
      (set `self.SQSoldier` _assqsoldier)
      ;[1 0 0] without delay it gains full velecity what ever what value you set DO NOT REMOVE
      (`KismetSystemLibrary.Delay` 0.2)
      (set `SQSoldier.FallingDamageMultiplier` 0.0 (`self.SQSoldier`))
      (set `MovementComponent.Velocity` (0.0 0.0 0.0) _charactermovement)
      (set `CharacterMovementComponent.GravityScale` 0.15 _charactermovement)
      (`NavMovementComponent.StopActiveMovement` _charactermovement)
      (`KismetSystemLibrary.PrintString` "using rope  " true true (struct :`G` 0.66 :`B` 1.0 :`A` 1.0) 10.0)
      ;[1 1 1] Will change here with basic delay after testing
      (bind _returnvalue (`KismetSystemLibrary.K2_SetTimerDelegate` (delegate `UpdateLocationToRope`) 0.07 false 0.03))
      ;[1 1 1] for observer it is should be not valid
      (`/Engine/EditorBlueprintResources/StandardMacros.IsValid` _asbp_player_controller
        (:`Is Valid`
          (`Controller.SetControlRotation` _asbp_player_controller (`SceneComponent.K2_GetComponentRotation` (`self.ComponentRefToFollow`)))
          (`Actor.DisableInput` _asbp_player_controller _asbp_player_controller)
          (`Controller.SetIgnoreLookInput` _asbp_player_controller true))
        (:`Is Not Valid`
          _))
      (bind _returnvalue_2 (`KismetSystemLibrary.K2_SetTimerDelegate` (delegate `check is landed`) 0.5 true)))
    (:`CastFailed`
      (`KismetSystemLibrary.PrintString` "SQSoldier cast failed  at fast rope component" true true (struct :`R` 1.0 :`B` 0.248225 :`A` 1.0) 20.0))))

(event `check is landed`
  (if (`NavMovementComponent.IsMovingOnGround` (`SQSoldier.SoldierMovement` (`self.SQSoldier`)))
    (`self.Deactivate`)))

(event `UpdateLocationToRope`
  (`self.SetComponentTickEnabled` true))

(event `self.ReceiveTick`
  (params (DeltaSeconds :type "Float (single-precision)"))
  (bind (_returnvalue_x _returnvalue_y _returnvalue_z) (`KismetMathLibrary.BreakVector` (`Actor.K2_GetActorLocation` (`self.SQSoldier`))))
  (bind (_returnvalue_x_2 _returnvalue_y_2) (`KismetMathLibrary.BreakVector` (`SceneComponent.K2_GetComponentLocation` (`self.ComponentRefToFollow`))))
  (`Actor.K2_SetActorLocation` (`self.SQSoldier`) (`KismetMathLibrary.MakeVector` (- _returnvalue_x_2 0.5) _returnvalue_y_2 _returnvalue_z) false false)
  (if (not (`/TestMod/TopFolder/SD_Heli/LatestBackup/BP_SD_Heli_Master_VersionERENEJ1.bRopeExist` (`self.HelicopterReference`)))
    (`self.Deactivate`)))

(fn `SetValuesForMovementCorrection`
  (params (inComponentRefToFollow :type "ArrowComponent Object Reference") (inHelicopterReference :type "/TestMod/TopFolder/SD_Heli/LatestBackup/BP_SD_Heli_Master_VersionERENEJ1 Object Reference"))
  (set `self.ComponentRefToFollow` inComponentRefToFollow)
  (set `self.HelicopterReference` inHelicopterReference))