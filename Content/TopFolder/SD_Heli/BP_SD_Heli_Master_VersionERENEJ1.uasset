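; Helicopter master Blueprint that adds four fast ropes for soldiers to rappel from a low, slow-moving helicopter.
; A looping timer checks velocity and altitude, detaching and hiding the ropes when limits are exceeded.
; LandingCamera activation drops the cables, using server-to-multicast events instead of variable replication to sync rope state.
; Soldiers leaving rope seats gain a movement-correction component following their exit point, and the server triggers their rappel.
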(event `self.ReceiveBeginPlay`
  ;[1 1 1] FastRopes
  (`parent.ReceiveBeginPlay`)
  ;;[1 1 1] begin play timer check for rope logic
  (`KismetSystemLibrary.K2_SetTimerDelegate` (delegate `Check Speed of Heli for rope`) 0.1 true))

(event `Check Speed of Heli for rope`
  (bind (_returnvalue_x _returnvalue_y _returnvalue_z) (`KismetMathLibrary.BreakVector` (`self.GetVelocity`)))
  ;[1 1 1] FastRopes
  ;;[1 1 1] begin play timer check for rope logic
  (bind _output_get (set `self.bHeliCanDropRope` (and (> _returnvalue_x -200.0) (< _returnvalue_x 200.0) (> _returnvalue_y -200.0) (< _returnvalue_y 200.0) (> _returnvalue_z -200.0) (< _returnvalue_z 200.0) (< (`self.Instruments-AltitudeMeters`) 30.0))))
  (if _output_get
    _
    (elif (`self.bRopeExist`)
      (`/Engine/EditorBlueprintResources/ActorMacros.Switch Has Authority`
        (:`Authority`
          (`self.MC_Detach and Hide the cable`))
        (:`Remote`
          (`self.SR_Detach and Hide the cable`))))))

(event `SR_Detach and Hide the cable`
  ;[1 1 1] FastRopes
  ;;[1 1 1] begin play timer check for rope logic
  (`self.MC_Detach and Hide the cable`))

(event `MC_Detach and Hide the cable`
  ;[1 1 1] FastRopes
  ;;[1 1 1] begin play timer check for rope logic
  (set `CableComponent.bAttachStart` false (`self.CableR`))
  (set `CableComponent.bAttachStart` false (`self.CableL`))
  (set `CableComponent.bAttachStart` false (`self.CableL1`))
  (set `CableComponent.bAttachStart` false (`self.CableR1`))
  (`KismetSystemLibrary.Delay` 0.25)
  (`SceneComponent.SetHiddenInGame` (`self.CableL`) true false)
  (`SceneComponent.SetHiddenInGame` (`self.CableR`) true false)
  (`SceneComponent.SetHiddenInGame` (`self.CableL1`) true false)
  (`SceneComponent.SetHiddenInGame` (`self.CableR1`) true false)
  (set `self.bRopeExist` false))

(event `MC_DropRopes`
  ;[1 1 1] FastRopes
  ;;[1 0.9023 0.1292] REPLICATION did NOT worked USED multicast instead there are value differences when detach cable bool called from inside bp and level bp it conflicts
  (set `CableComponent.bAttachStart` true (`self.CableR`))
  (set `CableComponent.bAttachStart` true (`self.CableL`))
  (set `CableComponent.bAttachStart` true (`self.CableL1`))
  (set `CableComponent.bAttachStart` true (`self.CableR1`))
  (`SceneComponent.SetHiddenInGame` (`self.CableL`) false false)
  (`SceneComponent.SetHiddenInGame` (`self.CableR`) false false)
  (`SceneComponent.SetHiddenInGame` (`self.CableL1`) false false)
  (`SceneComponent.SetHiddenInGame` (`self.CableR1`) false false)
  (`SceneComponent.K2_SetRelativeLocation` (`self.CableL`) (0.0 0.0 0.0) false false)
  (`SceneComponent.K2_SetRelativeLocation` (`self.CableR`) (0.0 0.0 0.0) false false)
  (`SceneComponent.K2_SetRelativeLocation` (`self.CableL1`) (0.0 0.0 0.0) false false)
  (`SceneComponent.K2_SetRelativeLocation` (`self.CableR1`) (0.0 0.0 0.0) false false)
  (`SceneComponent.K2_AttachToComponent` (`self.CableL`) (`self.CableStartPointL`) "Socket_FastRope_L" "KeepRelative" "KeepRelative" "KeepRelative" true)
  (`SceneComponent.K2_AttachToComponent` (`self.CableR`) (`self.CableStartPointR`) "Socket_FastRope_R" "KeepRelative" "KeepRelative" "KeepRelative" true)
  (`SceneComponent.K2_AttachToComponent` (`self.CableL1`) (`self.CableStartPointL1`) "Socket_FastRope_L" "KeepRelative" "KeepRelative" "KeepRelative" true)
  (`SceneComponent.K2_AttachToComponent` (`self.CableR1`) (`self.CableStartPointR1`) "Socket_FastRope_R" "KeepRelative" "KeepRelative" "KeepRelative" true)
  (`CableComponent.SetAttachEndTo` (`self.CableL`) null "EndpointRopeL" "None")
  (`CableComponent.SetAttachEndTo` (`self.CableR`) null "EndpointRopeR" "None")
  (`CableComponent.SetAttachEndTo` (`self.CableL1`) null "EndpointRopeL1" "None")
  (`CableComponent.SetAttachEndTo` (`self.CableR1`) null "EndpointRopeR1" "None")
  (set `self.bRopeExist` true))

(event `SR_DropRopes`
  ;[1 1 1] FastRopes
  ;;[1 0.9023 0.1292] REPLICATION did NOT worked USED multicast instead there are value differences when detach cable bool called from inside bp and level bp it conflicts
  (`self.MC_DropRopes`))

(event `self.LandingCamera.OnComponentActivated`
  (params (Component :type "ActorComponent Object Reference") (bReset :type Boolean))
  ;[1 1 1] FastRopes
  ;;[1 0.9023 0.1292] REPLICATION did NOT worked USED multicast instead there are value differences when detach cable bool called from inside bp and level bp it conflicts
  ;;;[1 1 1] when 'C' key pressed fires this nodes
  (if (`self.bHeliCanDropRope`)
    (`/Engine/EditorBlueprintResources/ActorMacros.Switch Has Authority`
      (:`Authority`
        (`self.MC_DropRopes`))
      (:`Remote`
        (`self.SR_DropRopes`)))))

(event `self.LeftVehicle`
  (params (Soldier :type "SQSoldier Object Reference") (PreviousSeat :type "SQVehicleSeatComponent Object Reference"))
  ;[1 1 1] FastRopes
  (`parent.LeftVehicle` Soldier PreviousSeat)
  (bind (_validropeseats _soldierpositioncomponent) (`self.SetRopeFollowingComponent` PreviousSeat))
  (if _validropeseats
    (`/Engine/EditorBlueprintResources/StandardMacros.IsValid` _soldierpositioncomponent
      (:`Is Valid`
        (bind _returnvalue (`AddComponent|NODE_AddBP_FastRopeComponent1-0` :`self` Soldier))
        (`ActorComponent.Activate` _returnvalue false)
        (`/TestMod/TopFolder/SD_Heli/LatestBackup/BP_FastRopeComponent1.SetValuesForMovementCorrection` _returnvalue _soldierpositioncomponent self)
        (`/Engine/EditorBlueprintResources/ActorMacros.Switch Has Authority`
          (:`Authority`
            (bind _assd_bp_mutable_soldier (cast `/Steel_Division/Blueprints/Mutablesoldiers/SD_BP_MutableSoldier` Soldier)
              (:`then`
                (`/Steel_Division/Blueprints/Mutablesoldiers/SD_BP_MutableSoldier.ServerSlotRappel` _assd_bp_mutable_soldier)
                (if (not (and (`ActorComponent.IsActive` _returnvalue) (`self.bRopeExist`)))
                  (`ActorComponent.Deactivate` _returnvalue)))
              (:`CastFailed`
                (`KismetSystemLibrary.PrintString` "Failed Cast of Soldier" true true (struct :`R` 1.0 :`G` 0.079394 :`A` 1.0))))))))))

(fn `SetHelicopterWidgetVisibilities`
  (params (InVisibility :type "ESlateVisibility Enum" :default "Visible"))
  (for _array_element (`SceneComponent.GetChildrenComponents` (`self.VehicleMesh`) true)
    (bind _aswidget_component (cast `WidgetComponent` _array_element))
    (`Widget.SetVisibility` (`WidgetComponent.GetUserWidgetObject` _aswidget_component) (`local.InVisibility`)))
  (return))

(fn `SetRopeFollowingComponent`
  (params (`Previous SQVehicleSeatComponent` :type "SQVehicleSeatComponent Object Reference"))
  (returns (ValidRopeSeats :type Boolean) (SoldierPositionComponent :type "ArrowComponent Object Reference"))
  (bind _returnvalue (== `Previous SQVehicleSeatComponent` (`|GetArrayItem` (`self.VehicleSeats`) 5)))
  (bind _returnvalue_2 (== `Previous SQVehicleSeatComponent` (`|GetArrayItem` (`self.VehicleSeats`) 6)))
  (bind _returnvalue_3 (== `Previous SQVehicleSeatComponent` (`|GetArrayItem` (`self.VehicleSeats`) 4)))
  (bind _returnvalue_4 (== `Previous SQVehicleSeatComponent` (`|GetArrayItem` (`self.VehicleSeats`) 7)))
  (bind _returnvalue_5 (and (or _returnvalue_3 _returnvalue _returnvalue_2 _returnvalue_4) (`self.bRopeExist`)))
  (if _returnvalue_3
    (return _returnvalue_5 (`self.ExitPointLeft`))
    (elif _returnvalue
      (return _returnvalue_5 (`self.ExitPointRight`))
      (elif _returnvalue_2
        (return _returnvalue_5 (`self.ExitPointLeft1`))
        (elif _returnvalue_4
          (return _returnvalue_5 (`self.ExitPointRight1`))
          (else
            (return false null)))))))

(fn `UserConstructionScript`
  (`parent.UserConstructionScript`))