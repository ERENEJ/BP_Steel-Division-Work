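; Javelin top-attack homing projectile that locks onto a ground vehicle and deals heavy anti-tank damage.
; It homes on a launch point, then a high target, before a looping timer steers it onto the vehicle mesh.
; Within 10m it simulates a hit by damaging and snapping to the vehicle, while box overlap handles other collisions.
; A replicated Exploded flag spawns the explosion effect; flare-decoy logic is present but disconnected.
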(event `self.ReceiveBeginPlay`
  (set `ProjectileMovementComponent.HomingTargetComponent` (`self.InitialLine`) (`self.ProjectileMovement`))
  (`KismetSystemLibrary.Delay` 0.5)
  (set `ProjectileMovementComponent.HomingTargetComponent` (`self.HightTarget`) (`self.ProjectileMovement`))
  (`KismetSystemLibrary.Delay` 3.0)
  (`ProjectileMovementComponent.SetVelocityInLocalSpace` (`self.ProjectileMovement`) (0.0 0.0 0.0))
  (`KismetSystemLibrary.PrintString` "is movement ok?" true true (struct :`R` 1.0 :`G` 0.200784 :`A` 1.0) 10.0)
  (bind _returnvalue (`KismetSystemLibrary.K2_SetTimerDelegate` (delegate `Lock on`) 0.1 true))
  (set `self.VehicleLockOnTimer` _returnvalue)
  ;[1 1 1] Flight time adjustment
  (`KismetSystemLibrary.Delay` 45.0)
  (`/Engine/EditorBlueprintResources/StandardMacros.IsValid` self
    (:`Is Valid`
      (`self.K2_DestroyActor`))))

(event `Lock on`
  (`/Engine/EditorBlueprintResources/StandardMacros.IsValid` (`self.TargetedGroundVehicle`)
    (:`Is Valid`
      (set `ProjectileMovementComponent.HomingTargetComponent` (`SQVehicle.VehicleMesh` (`self.TargetedGroundVehicle`)) (`self.ProjectileMovement`))
      (if (< (`KismetMathLibrary.Abs` (`KismetMathLibrary.Vector_Distance` (`SceneComponent.K2_GetComponentLocation` (`SQVehicle.VehicleMesh` (`self.TargetedGroundVehicle`))) (`self.K2_GetActorLocation`))) 1000.0)
        ;[1 1 1] method for preventing missile avoding vehicle at sharp turns this can be used simulated collision with missile
        (`GameplayStatics.ApplyDamage` (`self.TargetedGroundVehicle`) 1500.0 null null "/Game/Gameplay/DamageTypes/BP_HAT_DamageType.BP_HAT_DamageType_C")
        (`self.K2_SetActorLocation` (`SceneComponent.K2_GetComponentLocation` (`SQVehicle.VehicleMesh` (`self.TargetedGroundVehicle`))) true)
        (set `self.bExploded` true)
        (`self.ForceNetUpdate`)
        (`KismetSystemLibrary.K2_ClearAndInvalidateTimerHandle` (`self.VehicleLockOnTimer`))
        (`KismetSystemLibrary.Delay` 1.5)
        (`self.K2_DestroyActor`)
        (`KismetSystemLibrary.PrintString` "PROJECTILE ON VEHICLE SIMULATED" true true (struct :`R` 1.0 :`A` 1.0) 20.0)))))

(event `self.Box.OnComponentBeginOverlap`
  (params (OverlappedComponent :type "PrimitiveComponent Object Reference") (OtherActor :type "Actor Object Reference") (OtherComp :type "PrimitiveComponent Object Reference") (OtherBodyIndex :type Integer) (bFromSweep :type Boolean) (SweepResult :type "HitResult Structure (by ref)"))
  (bind _assqvehicle (cast `SQVehicle` OtherActor))
  (if (`self.bTargetedFlare`)
    (`self.K2_DestroyActor`)
    (else
      (`GameplayStatics.ApplyDamage` _assqvehicle 1500.0 null null "/Game/Gameplay/DamageTypes/BP_HAT_DamageType.BP_HAT_DamageType_C")
      (`KismetSystemLibrary.K2_ClearAndInvalidateTimerHandle` (`self.VehicleLockOnTimer`))
      (set `self.lastKnownVehicleLocation` (`self.K2_GetActorLocation`))
      (set `self.bExploded` true)
      (`self.ForceNetUpdate`)
      (`KismetSystemLibrary.Delay` 2.2)
      (`self.K2_DestroyActor`)
      (`KismetSystemLibrary.PrintString` "PROJECTILE COLLIDED WITH OTHER VEHICLE" true true (struct :`R` 0.961351 :`B` 1.0 :`A` 1.0) 20.0))))

(fn `OnRep_bExploded`
  (if (`self.bExploded`)
    (`/Engine/EditorBlueprintResources/StandardMacros.Can Execute Cosmetic Events`
      (:`True`
        (if (`self.bTargetedFlare`)
          (`|SpawnActorFromClass` "/Game/Blueprints/Effects/BP_LastingEffect_TOW.BP_LastingEffect_TOW_C" (`KismetMathLibrary.Conv_VectorToTransform` (`self.lastKnownVehicleLocation`)) "AlwaysSpawn" "OverrideRootScale" null null)
          (`KismetSystemLibrary.PrintString` "Targeted Flare" true true (struct :`G` 0.66 :`B` 1.0 :`A` 1.0) 20.0)
          (else
            (`|SpawnActorFromClass` "/Game/Blueprints/Effects/BP_LastingEffect_TOW.BP_LastingEffect_TOW_C" (`KismetMathLibrary.Conv_VectorToTransform` (`self.K2_GetActorLocation`)) "AlwaysSpawn" "OverrideRootScale" null null)
            (`KismetSystemLibrary.PrintString` "Targeted NOT Flare" true true (struct :`G` 0.66 :`B` 1.0 :`A` 1.0) 20.0)))))))

(fn `UserConstructionScript`)