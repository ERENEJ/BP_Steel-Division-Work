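; Javelin lock-on launcher weapon that fires guided projectiles at Squad ground vehicles.
; On fire, a delayed sphere trace from the barrel socket accepts a vehicle within a distance window, then shows the lock widget and plays sounds.
; Server events then spawn the projectile and assign its target.
; Failed locks on remote clients, and server-side unequips without a launch, reset the magazine to one round.
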(event `SR_CreateProjectileServer`
  (`/Engine/EditorBlueprintResources/ActorMacros.Switch Has Authority`
    (:`Authority`
      (bind _returnvalue (`|SpawnActorFromClass` "/TestMod/TopFolder/LockOnSystem/UpdatedCopy/BP_JavelineProjectile.BP_JavelineProjectile_C" (`SceneComponent.K2_GetComponentToWorld` (`self.Mesh3P`)) "AdjustIfPossibleButAlwaysSpawn" "OverrideRootScale" self null)) ; Spawn projectile
      (set `self.JavelineProjectile` _returnvalue)
      (`GameplayStatics.PlaySoundAtLocation` "/Game/Vehicles/BTR80/Sounds/Fire/2A72/Fire/1p/Initial/2A72_fire_1p_initial_start_01.2A72_fire_1p_initial_start_01" (`SceneComponent.K2_GetComponentLocation` (`self.Mesh1P`)) (struct) 1.0 1.0 0.0 null null null) ; Play firing sound
      (set `self.bWeaponFired` true))))

(event `ROC_AddAmmo`
  (bind (_defaultroundspermag _remainingrounds) (break `SQMagazineData` (`|GetArrayItem` (`self.Magazines`))))
  (`|VariableSetRef` _defaultroundspermag 1)
  (`|VariableSetRef` _remainingrounds 1)
  (`KismetSystemLibrary.PrintString` "rearmed  weapon" true true (struct :`G` 0.66 :`B` 1.0 :`A` 1.0) 20.0))

(event `SR_DesignateTarget`
  (params (Proj_Target :type "SQGroundVehicle Object Reference"))
  (bind _javelineprojectile (`self.JavelineProjectile`))
  (`/Engine/EditorBlueprintResources/ActorMacros.Switch Has Authority`
    (:`Authority`
      (`/Engine/EditorBlueprintResources/StandardMacros.IsValid` _javelineprojectile
        (:`Is Valid`
          (set `/TestMod/TopFolder/LockOnSystem/UpdatedCopy/BP_JavelineProjectile.TargetedGroundVehicle` Proj_Target _javelineprojectile))
        (:`Is Not Valid`
          (`KismetSystemLibrary.PrintString` "jav Projectile invalid" true true (struct :`G` 0.66 :`B` 1.0 :`A` 1.0) 20.0))))))

(event `SR_PlayJavelinSounds`
  (`|SpawnActorFromClass` "/TestMod/TopFolder/LockOnSystem/UpdatedCopy/BP_StingerSoundActor1.BP_StingerSoundActor1_C" (`self.GetTransform`) "Undefined" "OverrideRootScale" null null))

(event `self.BlueprintOnFire`
  (params (Origin :type "Vector Structure (by ref)"))
  (bind _mesh1p (`self.Mesh1P`))
  (set `self.bWeaponFired` false)
  (`GameplayStatics.PlaySoundAtLocation` null (`self.K2_GetActorLocation`) (struct) 1.0 1.0 2.0 "/Game/Audio/Attenuation/AkTestAttenuation/AkTestNearAttenuation.AkTestNearAttenuation" null null)
  (`KismetSystemLibrary.Delay` 1.0)
  (bind _outhit (`KismetSystemLibrary.SphereTraceSingle` (`SceneComponent.GetSocketLocation` (`self.Mesh1P`) "UGLBarrelStart") (+ (`SceneComponent.K2_GetComponentLocation` _mesh1p) (* (`KismetMathLibrary.GetForwardVector` (`SceneComponent.GetSocketRotation` _mesh1p "UGLBarrelStart")) 1500000.0)) 20.0 "TraceTypeQuery1" false (`|MakeArray` (`self.GetOwner`)) "ForDuration"))
  (if (and (< 12000.0 (`.Distance` (`GameplayStatics.BreakHitResult` _outhit))) (> 80000.0 (`.Distance` (`GameplayStatics.BreakHitResult` _outhit))))
    (bind _assqground_vehicle (cast `SQGroundVehicle` (`.HitActor` (`GameplayStatics.BreakHitResult` _outhit)))
      (:`then`
        (`SceneComponent.SetVisibility` (`self.LockedOnWidget`) true true)
        (`self.SR_PlayJavelinSounds`)
        (`KismetSystemLibrary.Delay` 1.0)
        (`parent.BlueprintOnFire` Origin)
        (`/Engine/EditorBlueprintResources/StandardMacros.IsValid` _assqground_vehicle
          (:`Is Valid`
            (`self.SR_CreateProjectileServer`)
            (`self.SR_DesignateTarget` _assqground_vehicle)
            (`KismetSystemLibrary.Delay` 2.0)
            (`SceneComponent.SetVisibility` (`self.LockedOnWidget`) false true))))
      (:`CastFailed`
        (`/Engine/EditorBlueprintResources/ActorMacros.Switch Has Authority` :!label _label
          (:`Remote`
            (`self.ROC_AddAmmo`)
            (set `self.bWeaponFired` false)))))
    (else
      (goto _label))))

(event `self.BlueprintOnUnequipped`
  (bind (_defaultroundspermag _remainingrounds) (break `SQMagazineData` (`|GetArrayItem` (`self.Magazines`))))
  (`parent.BlueprintOnUnequipped`)
  (`/Engine/EditorBlueprintResources/ActorMacros.Switch Has Authority`
    (:`Authority`
      (if (not (`self.bWeaponFired`))
        (`|VariableSetRef` _defaultroundspermag 1)
        (`|VariableSetRef` _remainingrounds 1)))))

(fn `UserConstructionScript`
  (`parent.UserConstructionScript`))