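; Stinger missile launcher weapon that locks onto helicopters and launches a guided projectile at them.
; On fire it plays a seeking sound, then after a delay sphere-traces from the barrel for a helicopter within a distance band.
; A hit triggers lock sounds, parent fire logic, and server events that spawn the projectile and assign its target.
; A failed lock restores the round on remote machines; unequipping without a launch rearms it on the server.
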(event `SR_CreateProjectileServer`
  (`/Engine/EditorBlueprintResources/ActorMacros.Switch Has Authority`
    (:`Authority`
      (bind _returnvalue (`|SpawnActorFromClass` "/TestMod/TopFolder/LockOnSystem/UpdatedCopy/BP_Stinger_Projectile.BP_Stinger_Projectile_C" (`SceneComponent.K2_GetComponentToWorld` (`self.Mesh3P`)) "AdjustIfPossibleButAlwaysSpawn" "OverrideRootScale" self null)) ; Spawn projectile
      (set `self.StingerProjectile` _returnvalue)
      (`GameplayStatics.PlaySoundAtLocation` "/Game/Vehicles/BTR80/Sounds/Fire/2A72/Fire/1p/Initial/2A72_fire_1p_initial_start_01.2A72_fire_1p_initial_start_01" (`SceneComponent.K2_GetComponentLocation` (`self.Mesh1P`)) (struct) 1.0 1.0 0.0 null null null) ; Play firing sound
      (set `self.bWeaponFired` true))))

(event `ROC_AddAmmo`
  (bind (_defaultroundspermag _remainingrounds) (break `SQMagazineData` (`|GetArrayItem` (`self.Magazines`))))
  (`|VariableSetRef` _defaultroundspermag 1)
  (`|VariableSetRef` _remainingrounds 1)
  (`KismetSystemLibrary.PrintString` "rearmed  weapon" true true (struct :`G` 0.66 :`B` 1.0 :`A` 1.0) 20.0))

(event `SR_DesignateTarget`
  (params (Proj_Target :type "/Game/Vehicles/UH60M/BP_Generic_Helicopter Object Reference"))
  (bind _stingerprojectile (`self.StingerProjectile`))
  (`/Engine/EditorBlueprintResources/ActorMacros.Switch Has Authority`
    (:`Authority`
      (`/Engine/EditorBlueprintResources/StandardMacros.IsValid` _stingerprojectile
        (:`Is Valid`
          (set `/TestMod/TopFolder/LockOnSystem/UpdatedCopy/BP_Stinger_Projectile.TargetedHelicopter` Proj_Target _stingerprojectile))
        (:`Is Not Valid`
          (`KismetSystemLibrary.PrintString` "Stinget Projectile invalid" true true (struct :`G` 0.66 :`B` 1.0 :`A` 1.0) 20.0))))))

(event `SR_PlayStingerSounds`
  (`|SpawnActorFromClass` "/TestMod/TopFolder/LockOnSystem/UpdatedCopy/BP_StingerSoundActor1.BP_StingerSoundActor1_C" (`self.GetTransform`) "Undefined" "OverrideRootScale" null null))

(event `self.BlueprintOnFire`
  (params (Origin :type "Vector Structure (by ref)"))
  (bind _mesh1p (`self.Mesh1P`))
  (set `self.bWeaponFired` false)
  (`KismetSystemLibrary.PrintString` "wep fire is false" true true (struct :`R` 1.0 :`G` 0.050478 :`A` 1.0) 20.0)
  (`GameplayStatics.PlaySoundAtLocation` "/Steel_Division/Blueprints/Weapons/RocketLaunchers/9K32M/Missile_target_Seeking_Cue.Missile_target_Seeking_Cue" (`self.K2_GetActorLocation`) (struct) 1.0 1.0 2.0 "/Game/Audio/Attenuation/AkTestAttenuation/AkTestNearAttenuation.AkTestNearAttenuation" null null)
  (`KismetSystemLibrary.Delay` 1.0)
  (bind _outhit (`KismetSystemLibrary.SphereTraceSingle` :`Start` (`SceneComponent.GetSocketLocation` (`self.Mesh1P`) "UGLBarrelStart") :`End` (+ (`SceneComponent.K2_GetComponentLocation` _mesh1p) (* (`KismetMathLibrary.GetForwardVector` (`SceneComponent.GetSocketRotation` _mesh1p "UGLBarrelStart")) 1500000.0)) :`Radius` 20.0 :`TraceChannel` "TraceTypeQuery1" :`DrawDebugType` "ForDuration"))
  (if (and (< 8000.0 (`.Distance` (`GameplayStatics.BreakHitResult` _outhit))) (> 100000.0 (`.Distance` (`GameplayStatics.BreakHitResult` _outhit))))
    (bind _asbp_generic_helicopter (cast `/Game/Vehicles/UH60M/BP_Generic_Helicopter` (`.HitActor` (`GameplayStatics.BreakHitResult` _outhit)))
      (:`then`
        (`self.SR_PlayStingerSounds`)
        (`KismetSystemLibrary.Delay` 1.0)
        (`parent.BlueprintOnFire` Origin)
        (`/Engine/EditorBlueprintResources/StandardMacros.IsValid` _asbp_generic_helicopter
          (:`Is Valid`
            (`self.SR_CreateProjectileServer`)
            (`self.SR_DesignateTarget` _asbp_generic_helicopter))))
      (:`CastFailed`
        (`/Engine/EditorBlueprintResources/ActorMacros.Switch Has Authority` :!label _label
          (:`Remote`
            (`self.ROC_AddAmmo`)
            (set `self.bWeaponFired` false)))))
    (else
      (goto _label))))

(event `self.BlueprintOnUnequipped`
  (bind (_defaultroundspermag _remainingrounds) (break `SQMagazineData` (`|GetArrayItem` (`self.Magazines`))))
  (`parent.BlueprintOnUnequipped`)
  (`/Engine/EditorBlueprintResources/ActorMacros.Switch Has Authority`
    (:`Authority`
      (if (not (`self.bWeaponFired`))
        (`|VariableSetRef` _defaultroundspermag 1)
        (`|VariableSetRef` _remainingrounds 1)))))

(fn `UserConstructionScript`)