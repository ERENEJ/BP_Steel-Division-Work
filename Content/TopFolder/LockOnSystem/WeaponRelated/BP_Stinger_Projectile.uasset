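; Stinger homing missile that tracks a targeted helicopter through a looping lock-on timer, triggering its missile warning.
; Within a short radius it simulates a hit, applying HAT damage and snapping onto the target to avoid misses on sharp turns; vehicle overlaps also deal damage.
; Fired flares stop tracking, causing delayed radial damage at the helicopter's last known position.
; The replicated Exploded flag's OnRep spawns the cosmetic explosion effect.
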(event `self.ReceiveBeginPlay`
  (bind _returnvalue (`KismetSystemLibrary.K2_SetTimerDelegate` (delegate `Lock on`) 0.1 true))
  (set `self.VehicleLockOnTimer` _returnvalue)
  ;[1 1 1] Flight time adjustment
  (`KismetSystemLibrary.Delay` 35.0)
  (`/Engine/EditorBlueprintResources/StandardMacros.IsValid` self
    (:`Is Valid`
      (`self.K2_DestroyActor`))))

(event `Lock on`
  (bind _returnvalue (`self.GetComponentByClass` (`self.TargetedHelicopter`) "/Steel_Division/Settings/Vehicles/CounterMeasures/BP_FlareLauncherComponent.BP_FlareLauncherComponent_C"))
  (bind _returnvalue_2 (`KismetMathLibrary.Conv_IntToDouble` (`KismetMathLibrary.Round` (/ (`KismetMathLibrary.Abs` (`KismetMathLibrary.Vector_Distance` (`self.lastKnownVehicleLocation`) (`self.K2_GetActorLocation`))) (`ProjectileMovementComponent.MaxSpeed` (`self.ProjectileMovement`))))))
  (`/Engine/EditorBlueprintResources/StandardMacros.IsValid` (`self.TargetedHelicopter`)
    (:`Is Valid`
      (`/Engine/EditorBlueprintResources/StandardMacros.IsValid` _returnvalue
        (:`Is Valid`
          (if (not (`/Steel_Division/Settings/Vehicles/CounterMeasures/BP_FlareLauncherComponent.FlaresFired` _returnvalue))
            (`/Steel_Division/Settings/Vehicles/CounterMeasures/BP_FlareLauncherComponent.SR_PlayMissileWarningSound` _returnvalue)
            (set `ProjectileMovementComponent.HomingTargetComponent` (`SQVehicle.VehicleMesh` (`self.TargetedHelicopter`)) (`self.ProjectileMovement`) :!label _label)
            (if (< (`KismetMathLibrary.Abs` (`KismetMathLibrary.Vector_Distance` (`SceneComponent.K2_GetComponentLocation` (`SQVehicle.VehicleMesh` (`self.TargetedHelicopter`))) (`self.K2_GetActorLocation`))) 1500.0)
              ;[1 1 1] method for preventing missile avoding vehicle at sharp turns this can be used simulated collision with missile
              (`GameplayStatics.ApplyDamage` (`self.TargetedHelicopter`) 2500.0 null null "/Game/Gameplay/DamageTypes/BP_HAT_DamageType.BP_HAT_DamageType_C")
              (`self.K2_SetActorLocation` (`SceneComponent.K2_GetComponentLocation` (`SQVehicle.VehicleMesh` (`self.TargetedHelicopter`))) true)
              (set `self.bExploded` true)
              (`self.ForceNetUpdate`)
              (`KismetSystemLibrary.K2_ClearAndInvalidateTimerHandle` (`self.VehicleLockOnTimer`))
              (`KismetSystemLibrary.Delay` 1.5)
              (`self.K2_DestroyActor`)
              (`KismetSystemLibrary.PrintString` "PROJECTILE ON VEHICLE SIMULATED" true true (struct :`R` 1.0 :`A` 1.0) 20.0))
            (else
              (set `self.lastKnownVehicleLocation` (`SceneComponent.K2_GetComponentLocation` (`SQVehicle.VehicleMesh` (`self.TargetedHelicopter`))))
              (set `self.bTargetedFlare` true)
              (`KismetSystemLibrary.K2_ClearAndInvalidateTimerHandle` (`self.VehicleLockOnTimer`))
              (`KismetSystemLibrary.PrintString` "This is projectile and I will be moved last position of vehicle " true true (struct :`R` 1.0 :`G` 0.134102 :`A` 1.0) 20.0)
              (`KismetSystemLibrary.PrintString` (`KismetStringLibrary.Concat_StrStr` "Projectile will destroy it self in " (`KismetStringLibrary.Conv_DoubleToString` _returnvalue_2)) true true (struct :`R` 1.0 :`G` 0.062616 :`B` 0.293968 :`A` 1.0) 20.0)
              (`KismetSystemLibrary.Delay` _returnvalue_2)
              (`GameplayStatics.ApplyRadialDamageWithFalloff` :`BaseDamage` 50.0 :`MinimumDamage` 10.0 :`Origin` (`self.lastKnownVehicleLocation`) :`DamageInnerRadius` 30.0 :`DamageOuterRadius` 50.0 :`DamageFalloff` 10.0 :`DamageTypeClass` "/Game/Gameplay/DamageTypes/BP_BasicHeatDamageType.BP_BasicHeatDamageType_C" :`DamageCauser` null :`InstigatedByController` null)
              (set `self.bExploded` true)
              (`self.ForceNetUpdate`)
              (`KismetSystemLibrary.Delay` 2.0)
              (`self.K2_DestroyActor`)
              (`KismetSystemLibrary.PrintString` "PROJECTILE MOVED FLARE LOCATION" true true (struct :`R` 1.0 :`A` 1.0) 20.0))))
        (:`Is Not Valid`
          (goto _label))))))

(event `self.Box.OnComponentBeginOverlap`
  (params (OverlappedComponent :type "PrimitiveComponent Object Reference") (OtherActor :type "Actor Object Reference") (OtherComp :type "PrimitiveComponent Object Reference") (OtherBodyIndex :type Integer) (bFromSweep :type Boolean) (SweepResult :type "HitResult Structure (by ref)"))
  (bind _assqvehicle (cast `SQVehicle` OtherActor))
  (if (`self.bTargetedFlare`)
    (`self.K2_DestroyActor`)
    (else
      (`GameplayStatics.ApplyDamage` _assqvehicle 2500.0 null null "/Game/Gameplay/DamageTypes/BP_HAT_DamageType.BP_HAT_DamageType_C")
      (`KismetSystemLibrary.K2_ClearAndInvalidateTimerHandle` (`self.VehicleLockOnTimer`))
      (set `self.lastKnownVehicleLocation` (`self.K2_GetActorLocation`))
      (set `self.bExploded` true)
      (`self.ForceNetUpdate`)
      (`KismetSystemLibrary.Delay` 2.2)
      (`self.K2_DestroyActor`)
      (`KismetSystemLibrary.PrintString` "PROJECTILE COLLIDED WITH OTHER VEHICLE" true true (struct :`R` 0.961351 :`B` 1.0 :`A` 1.0) 20.0))))

(event `self.CollisionComp.OnComponentHit`
  (params (HitComponent :type "PrimitiveComponent Object Reference") (OtherActor :type "Actor Object Reference") (OtherComp :type "PrimitiveComponent Object Reference") (NormalImpulse :type "Vector Structure") (Hit :type "HitResult Structure (by ref)"))
  (`KismetSystemLibrary.Delay` 4.0)
  (`/Engine/EditorBlueprintResources/StandardMacros.IsValid` self
    (:`Is Valid`
      (`self.K2_DestroyActor`))))

(fn `OnRep_bExploded`
  (if (`self.bExploded`)
    (`/Engine/EditorBlueprintResources/StandardMacros.Can Execute Cosmetic Events`
      (:`True`
        (if (`self.bTargetedFlare`)
          (`|SpawnActorFromClass` "/Game/Blueprints/Effects/BP_LastingEffect_TOW.BP_LastingEffect_TOW_C" (`KismetMathLibrary.Conv_VectorToTransform` (`self.lastKnownVehicleLocation`)) "AlwaysSpawn" "OverrideRootScale" null null)
          (`KismetSystemLibrary.PrintString` "Targeted Flare" true true (struct :`G` 0.66 :`B` 1.0 :`A` 1.0) 20.0)
          (else
            (`|SpawnActorFromClass` "/Game/Blueprints/Effects/BP_LastingEffect_TOW.BP_LastingEffect_TOW_C" (`KismetMathLibrary.Conv_VectorToTransform` (`self.K2_GetActorLocation`)) "AlwaysSpawn" "OverrideRootScale" null null)
            (`KismetSystemLibrary.PrintString` "Targeted NOT Flare" true true (struct :`G` 0.66 :`B` 1.0 :`A` 1.0) 20.0)))))))

(fn `UserConstructionScript`)