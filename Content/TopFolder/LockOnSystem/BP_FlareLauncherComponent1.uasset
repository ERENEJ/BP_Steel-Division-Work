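; Flare launcher scene component for the lock-on system that fires countermeasure flare bursts and plays missile warning audio.
; FireFlares loops through a delayed burst, spawning BP_Flare at the component's transform with a launch sound, then resets its counter.
; FlaresFired is raised during each delay, and a debug message says the target becomes targetable when the sequence ends.
; SR_PlayMissileWarningSound forwards the component's location to the warning sound event, with origin-rebased playback.
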(event `FireFlares`
  (`KismetSystemLibrary.PrintString` " flare launcher  called it will be  targetable when flare squence is finished" true true (struct :`G` 0.66 :`B` 1.0 :`A` 1.0) 20.0)
  (if (> (`self.FlareBurstLength`) (`self.CurrentFlareBurstLength`)) :!label _label
    (`|SpawnActorFromClass` "/Steel_Division/Settings/Vehicles/CounterMeasures/BP_Flare.BP_Flare_C" (`self.K2_GetComponentToWorld`) "AlwaysSpawn" "OverrideRootScale" null null)
    (`self.PlayFlareSounds` (`self.K2_GetComponentLocation`))
    (set `self.FlaresFired` true)
    (`KismetSystemLibrary.Delay` (`self.FlareDelay`))
    (`/Engine/EditorBlueprintResources/StandardMacros.IncrementInt` (`self.CurrentFlareBurstLength`)
      (:`  `
        (set `self.FlaresFired` false)
        (goto _label)))
    (else
      (set `self.CurrentFlareBurstLength` 0))))

(event `PlayFlareSounds`
  (params (Location :type "Vector Structure"))
  (`GameplayStatics.PlaySoundAtLocation` (`self.FlareLaunchSound`) (`GameplayStatics.RebaseZeroOriginOntoLocal` Location) (struct) 1.0 1.0 0.0 null null null))

(event `SR_PlayMissileWarningSound`
  (`self.PlayMissileWarningSound` (`self.K2_GetComponentLocation`)))

(event `PlayMissileWarningSound`
  (params (WorldLocation :type "Vector Structure"))
  (`GameplayStatics.PlaySoundAtLocation` (`self.MissileWarningSound`) (`GameplayStatics.RebaseZeroOriginOntoLocal` WorldLocation) (struct) 1.0 1.0 0.0 "/Game/Audio/Attenuation/AkTestAttenuation/AkTestMidAttenuation.AkTestMidAttenuation" null null))