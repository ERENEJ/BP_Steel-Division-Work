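; BP_DayOrNight is an actor that switches the map's lighting setup by streaming either the Anvil mid-day level or the night level.
; On BeginPlay it calls SR_DecideDay, which waits briefly, then reads DayOrNight to unload one sublevel and load the other without blocking.
; A true DayOrNight selects night.
; The variable has a RepNotify, but its handler does nothing, so later changes do not trigger a switch by themselves.
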(event `SR_DecideDay`
  (`KismetSystemLibrary.Delay` 3.0)
  (if (`self.DayOrNight`)
    (`GameplayStatics.UnloadStreamLevel` "/TestMod/TopFolder/Maps/LL_Anvil_Mid_Day")
    (`GameplayStatics.LoadStreamLevel` "/TestMod/TopFolder/Maps/SD_LL_Night" true)
    (else
      (`GameplayStatics.UnloadStreamLevel` "/TestMod/TopFolder/Maps/SD_LL_Night")
      (`GameplayStatics.LoadStreamLevel` "/TestMod/TopFolder/Maps/LL_Anvil_Mid_Day" true))))

(event `self.ReceiveBeginPlay`
  (`self.SR_DecideDay`))

(fn `OnRep_DayOrNight`)

(fn `UserConstructionScript`)