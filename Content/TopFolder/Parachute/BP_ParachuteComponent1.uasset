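; Actor component that runs a parachute jump for a mutable soldier, from freefall to landing.
; On activation it boosts air control, then looping timers check the drop below VehicleAltitude to open the chute and detect ground contact.
; SR events sequence animation states with delays and spawn, attach or delete the parachute mesh actor.
; Deployment cuts gravity and fall damage; landing sets movement values back, and the component self-destroys afterwards or 60 seconds after BeginPlay.
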(event `SR_DeleteAttachedParachute`
  (bind _parachutemeshactor (`self.ParachuteMeshActor`))
  (`/Engine/EditorBlueprintResources/StandardMacros.IsValid` _parachutemeshactor
    (:`Is Valid`
      (`Actor.K2_DetachFromActor` _parachutemeshactor "KeepRelative" "KeepRelative" "KeepRelative")
      (`Actor.K2_DestroyActor` _parachutemeshactor))))

(event `SR_SpawnAndAttachParachute`
  (params (SD_MutableSoldier :type "/Steel_Division/Blueprints/Mutablesoldiers/SD_BP_MutableSoldier Object Reference"))
  (bind _returnvalue (`|SpawnActorFromClass` "/TestMod/TopFolder/Parachute/LatestVersion/BP_Parachute_Meshes1.BP_Parachute_Meshes1_C" (`Actor.GetTransform` SD_MutableSoldier) "AlwaysSpawn" "OverrideRootScale" null null))
  (`/Engine/EditorBlueprintResources/StandardMacros.IsValid` _returnvalue
    (:`Is Valid`
      (bind _output_get (set `self.ParachuteMeshActor` _returnvalue))
      (`SceneComponent.K2_AttachToComponent` (`Actor.RootComponent` _output_get) (`Character.Mesh` SD_MutableSoldier) "Bip01_Spine" "SnapToTarget" "KeepWorld" "KeepWorld" false))))

(event `self.ReceiveBeginPlay`
  (add `self.OnComponentActivated` (delegate `OnActivate`))
  (`KismetSystemLibrary.Delay` 60.0)
  (`self.Deactivate`)
  (`self.K2_DestroyComponent`))

(event `OnActivate` :!signature `self.OnComponentActivated`
  (params (Component :type "ActorComponent Object Reference") (bReset :type Boolean))
  (bind _assd_bp_mutable_soldier (cast `/Steel_Division/Blueprints/Mutablesoldiers/SD_BP_MutableSoldier` (`self.GetOwner` Component))
    (:`then`
      (`self.SR_Parachute jump` _assd_bp_mutable_soldier)
      (bind _charactermovement (`Character.CharacterMovement` _assd_bp_mutable_soldier))
      (set `CharacterMovementComponent.MaxFlySpeed` 1999999991808.0 _charactermovement)
      (set `CharacterMovementComponent.AirControl` 1999999973982208.0 _charactermovement)
      (set `CharacterMovementComponent.AirControlBoostMultiplier` 1999999991808.0 _charactermovement)
      (set `CharacterMovementComponent.AirControlBoostVelocityThreshold` 1999999991808.0 _charactermovement)
      (`KismetSystemLibrary.PrintString` "there must be falling anim right now!" true true (struct :`R` 1.0 :`G` 0.027472 :`A` 1.0) 10.0)
      (bind _returnvalue (`KismetSystemLibrary.K2_SetTimerDelegate` (delegate `Check Player Altidute`) 2.0 true)))
    (:`CastFailed`
      (`KismetSystemLibrary.PrintString` "SD Mutable soldier cast failed" true true (struct :`R` 1.0 :`G` 0.027472 :`A` 1.0) 10.0))))

(event `Check Player Altidute`
  (bind (_returnvalue_x _returnvalue_y _returnvalue_z) (`KismetMathLibrary.BreakVector` (`SceneComponent.K2_GetComponentLocation` (`Actor.RootComponent` (stale `OnActivate` _assd_bp_mutable_soldier)))))
  (if (> (- (`self.VehicleAltitude`) _returnvalue_z) 60000.0)
    (`self.SR_Call for Parachute to deploy` (stale `OnActivate` _assd_bp_mutable_soldier))
    (`self.SR_SpawnAndAttachParachute` (stale `OnActivate` _assd_bp_mutable_soldier))
    (set `SQSoldier.FallingDamageMultiplier` 0.0 (stale `OnActivate` _assd_bp_mutable_soldier))
    (bind _charactermovement (`Character.CharacterMovement` (stale `OnActivate` _assd_bp_mutable_soldier)))
    (set `MovementComponent.Velocity` (0.0 0.0 0.0) _charactermovement)
    ;[1 1 1] it was 0.4 before
    (set `CharacterMovementComponent.GravityScale` 0.2 _charactermovement)
    (`NavMovementComponent.StopActiveMovement` _charactermovement)
    (`KismetSystemLibrary.K2_ClearAndInvalidateTimerHandle` (stale `OnActivate` _returnvalue))
    (`KismetSystemLibrary.PrintString` "open parachute func " true true (struct :`G` 0.66 :`B` 1.0 :`A` 1.0) 10.0)
    (bind _returnvalue (`KismetSystemLibrary.K2_SetTimerDelegate` (delegate `check is landed`) 1.0 true))))

(event `check is landed`
  (if (`NavMovementComponent.IsMovingOnGround` (`SQSoldier.SoldierMovement` (stale `OnActivate` _assd_bp_mutable_soldier)))
    (`self.SR_ Server Landing` (stale `OnActivate` _assd_bp_mutable_soldier))
    (set `MovementComponent.Velocity` (0.0 0.0 0.0) (`SQSoldier.SoldierMovement` (stale `OnActivate` _assd_bp_mutable_soldier)))
    (`KismetSystemLibrary.PrintString` "there must be landing anim right now" true true (struct :`R` 1.0 :`G` 0.027472 :`A` 1.0))
    (bind _charactermovement (`Character.CharacterMovement` (stale `OnActivate` _assd_bp_mutable_soldier)))
    (`NavMovementComponent.StopActiveMovement` _charactermovement)
    (set `CharacterMovementComponent.GravityScale` 1.0 _charactermovement)
    (set `SQSoldier.FallingDamageMultiplier` 50.0 (stale `OnActivate` _assd_bp_mutable_soldier))
    (set `CharacterMovementComponent.MaxFlySpeed` 200.0 _charactermovement)
    (set `CharacterMovementComponent.AirControl` 0.05 _charactermovement)
    (set `CharacterMovementComponent.AirControlBoostMultiplier` 2.0 _charactermovement)
    (set `CharacterMovementComponent.AirControlBoostVelocityThreshold` 25.0 _charactermovement)
    (set `CharacterMovementComponent.JumpZVelocity` 310.0 _charactermovement)
    (set `CharacterMovementComponent.BrakingDecelerationFalling` 0.0 _charactermovement)
    (set `CharacterMovementComponent.FallingLateralFriction` 0.0 _charactermovement)
    (`KismetSystemLibrary.K2_ClearAndInvalidateTimerHandle` (stale `Check Player Altidute` _returnvalue))
    (`KismetSystemLibrary.PrintString` "soldier is landing" true true (struct :`R` 1.0 :`A` 1.0) 20.0)
    (`self.SR_DeleteAttachedParachute`)
    (`KismetSystemLibrary.Delay` 8.0)
    (`self.Deactivate`)
    (`self.K2_DestroyComponent`)))

(event `SR_Parachute jump`
  (params (Target :type "/Steel_Division/Blueprints/Mutablesoldiers/SD_BP_MutableSoldier Object Reference"))
  ;[1 1 1] Initial Parachute Jump to Fall
  (`/Steel_Division/Blueprints/Mutablesoldiers/SD_BP_MutableSoldier.Server Is Jump to Fall` Target)
  ;;[1 1 1] Animation Timer Dont change
  (`KismetSystemLibrary.Delay` 1.6)
  (`/Steel_Division/Blueprints/Mutablesoldiers/SD_BP_MutableSoldier.Server Is Fall Idle` Target))

(event `SR_Call for Parachute to deploy`
  (params (Target :type "/Steel_Division/Blueprints/Mutablesoldiers/SD_BP_MutableSoldier Object Reference"))
  ;[1 1 1] Parachute Deploying
  (`KismetSystemLibrary.Delay` 1.0)
  (`/Steel_Division/Blueprints/Mutablesoldiers/SD_BP_MutableSoldier.Server Is Fall to Deploy` Target)
  ;;[1 1 1] Animation Timer Dont Change
  (`KismetSystemLibrary.Delay` 1.6)
  (`/Steel_Division/Blueprints/Mutablesoldiers/SD_BP_MutableSoldier.Server Is Deploy Idle` Target))

(event `SR_ Server Landing`
  (params (Target :type "/Steel_Division/Blueprints/Mutablesoldiers/SD_BP_MutableSoldier Object Reference"))
  ;[1 1 1] Parachute Landing
  (`KismetSystemLibrary.Delay` 1.0)
  (`/Steel_Division/Blueprints/Mutablesoldiers/SD_BP_MutableSoldier.Server Is Deploy to Landing` Target)
  ;;[1 1 1] Animation Timer Dont Change
  (`KismetSystemLibrary.Delay` 3.0)
  (`/Steel_Division/Blueprints/Mutablesoldiers/SD_BP_MutableSoldier.Server Is Landed` Target)
  (`KismetSystemLibrary.Delay` 1.0))